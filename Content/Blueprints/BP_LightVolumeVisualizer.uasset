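; Debug-style actor that displays the light (shadow) volume of an assigned raymarched volume on its static mesh.
; On BeginPlay it creates a dynamic instance of the mesh material and feeds it the volume's ALightVolume texture, or prints a warning if no volume is set.
; It copies the volume's scale and rotation at start and every Tick, leaving its own location independent.
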(event Collision|EventActorBeginOverlap
  (params (OtherActor :type Actor%20Object%20Reference)))

(event EventTick
  (params (DeltaSeconds :type Float%20%28single-precision%29))
  (bind _raymarched_volume_to_visualize_shadow_for (Variables|Default|GetRaymarched%20Volume%20To%20Visualize%20Shadow%20For))
  (Utilities|IsValid _raymarched_volume_to_visualize_shadow_for
    (:Is%20Valid
      (Transformation|SetActorScale3D (Transformation|GetActorScale3D _raymarched_volume_to_visualize_shadow_for))
      (Transformation|SetActorRotation (Transformation|GetActorRotation _raymarched_volume_to_visualize_shadow_for)))))

(event EventBeginPlay
  (bind _staticmeshcomponent (Variables|Debug|GetStaticMeshComponent))
  (bind _raymarched_volume_to_visualize_shadow_for (Variables|Default|GetRaymarched%20Volume%20To%20Visualize%20Shadow%20For))
  (bind _returnvalue (Rendering|Material|GetMaterial _staticmeshcomponent 0))
  (Utilities|IsValid _raymarched_volume_to_visualize_shadow_for
    (:Is%20Valid
      (Transformation|SetActorScale3D (Transformation|GetActorScale3D _raymarched_volume_to_visualize_shadow_for))
      (Transformation|SetActorRotation (Transformation|GetActorRotation _raymarched_volume_to_visualize_shadow_for))
      (bind _returnvalue_2 (Rendering|Material|CreateDynamicMaterialInstance _returnvalue (Utilities|String|StringToName (Utilities|String|Append (Utilities|GetObjectName _returnvalue) "_Dynamic")) :!class /Script/Engine.KismetMaterialLibrary))
      (bind _output_get (Variables|Default|SetDynamic%20Visualize%20Material _returnvalue_2))
      (Rendering|Material|SetMaterial (Variables|Debug|GetStaticMeshComponent) 0 _output_get)
      (Rendering|Material|SetTextureParameterValue (Variables|Default|GetDynamic%20Visualize%20Material) "ALightVolume" (Variables|/Raymarcher/Blueprints/BP_RaymarchedVolume.BP_RaymarchedVolume_C|GetALightVolume (Variables|Default|GetRaymarched%20Volume%20To%20Visualize%20Shadow%20For))))
    (:Is%20Not%20Valid
      (Development|PrintString "Light Volume Visualizer doesn't have a Raymarch Volume Set!" true true "(R=1.000000,G=0.066208,B=0.000000,A=1.000000)" 1e+01))))

(fn ConstructionScript)