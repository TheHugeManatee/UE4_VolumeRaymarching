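; BP_RaymarchingLight is a directional light actor that supplies direction and intensity parameters for raymarched lighting.
; Its forward vector serves as the light direction, packed with LightIntensity into DirLightParameters.
; It caches the previous direction and intensity, so NeedsUpdate can flag changes, using a small tolerance for direction.
; The event graph holds only disconnected legacy mouse-rotation logic, which never runs.
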(event EventBeginPlay
  ;[1 1 1] Legacy
)

(event Collision|EventActorBeginOverlap
  (params (OtherActor :type Actor%20Object%20Reference)))

(event EventTick
  (params (DeltaSeconds :type Float%20%28single-precision%29)))

(event Input|AxisEvents|InputAxisMouseRotationX
  (params (AxisValue :type Float%20%28single-precision%29))
  ;[1 1 1] Legacy
)

(event Input|AxisEvents|InputAxisMouseRotationY
  (params (AxisValue :type Float%20%28single-precision%29))
  ;[1 1 1] Legacy
)

(fn ConstructionScript)

(fn GetCurrent
  (return (Utilities|Struct|MakeDirLightParameters (Transformation|GetActorForwardVector) (Variables|Default|GetLight%20Intensity))))

(fn SetPrevious
  (params (Light%20Parameters :type Dir%20Light%20Parameters%20Structure))
  (bind (_lightdirection _lightintensity) (Utilities|Struct|BreakDirLightParameters Light%20Parameters))
  (Variables|Default|SetLast%20Direction _lightdirection)
  (Variables|Default|SetLast%20Light%20Intensity _lightintensity))

(fn GetPrevious
  (return (Utilities|Struct|MakeDirLightParameters (Variables|Default|GetLast%20Direction) (Variables|Default|GetLast%20Light%20Intensity))))

(fn SetCurrentasPrevious
  (Variables|Default|SetLast%20Direction (Transformation|GetActorForwardVector))
  (Variables|Default|SetLast%20Light%20Intensity (Variables|Default|GetLight%20Intensity)))

(fn NeedsUpdate
  (return (or (Math|Vector|NotEqual(Vector) (Transformation|GetActorForwardVector) (Variables|Default|GetLast%20Direction) 0.0001) (!= (Variables|Default|GetLight%20Intensity) (Variables|Default|GetLast%20Light%20Intensity)))))