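; BP_ClippingPlane is a movable plane actor that defines a clipping cut from its location and up vector, clipping away the down side.
; Its construction script builds a bordered dynamic material, while helper functions track previous parameters to report when the cut needs updating.
; An input action toggles visibility, parking the hidden plane high up and restoring its last visible transform.
; The screen-material setup in the event graph is unconnected and never runs.
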(event EventBeginPlay)

(event Collision|EventActorBeginOverlap
  (params (OtherActor :type Actor%20Object%20Reference)))

(event EventTick
  (params (DeltaSeconds :type Float%20%28single-precision%29)))

(event Input|ActionEvents|InputActionClippingPlaneVisibilitySwitch
  (params (Key :type Key%20Structure))
  ;[1 1 1] To be moved to pickup_clip_with_screen, once the material is clean for that
  (:Pressed
    (CallFunction|ToggleVisibility)))

(fn ConstructionScript
  (Variables|Default|SetOldParameters (Utilities|Struct|MakeClippingPlaneParameters (Transformation|GetActorLocation) (Transformation|GetActorUpVector)))
  (Rendering|Material|SetMaterial (Variables|Default|GetClippingPlane) 0 (Rendering|Material|GetMaterial (Variables|Debug|GetStaticMeshComponent) 0))
  ;[0 0 0] Make dynamic material for the clipping plane and set parameters
  (bind _returnvalue (Rendering|Material|CreateDynamicMaterialInstance (Variables|Default|GetClippingPlane) 0 (Rendering|Material|GetMaterial (Variables|Debug|GetStaticMeshComponent) 0) "Standard" :!class /Script/Engine.PrimitiveComponent))
  (bind _output_get (Variables|Default|SetMyMat _returnvalue))
  (Rendering|Material|SetScalarParameterValue _output_get "BorderWidth" (Variables|Default|GetBorderThickness) :!class /Script/Engine.MaterialInstanceDynamic)
  (Rendering|Material|SetVectorParameterValue (Variables|Default|GetMyMat) "BorderColor" (Math|Conversions|ToLinearColor(Color) (Variables|Default|GetBorderColor)) :!class /Script/Engine.MaterialInstanceDynamic)
  (Rendering|Material|SetScalarParameterValue (Variables|Default|GetMyMat) "BrightnessThreshold" 1.1 :!class /Script/Engine.MaterialInstanceDynamic))

(fn GetCurrentParameters
  (return (Utilities|Struct|MakeClippingPlaneParameters (Transformation|GetActorLocation) (* (Transformation|GetActorUpVector) -1.0))))

(fn NeedsUpdate
  (bind _clippingcenter (CallFunction|GetCurrentParameters))
  (bind _oldparameters (Variables|Default|GetOldParameters))
  (bind (_center _direction) (Utilities|Struct|BreakClippingPlaneParameters _oldparameters))
  (bind (_center_2 _direction_2) (Utilities|Struct|BreakClippingPlaneParameters _clippingcenter))
  (return (or (Math|Vector|NotEqual(Vector) _center_2 _center 0.0001) (Math|Vector|NotEqual(Vector) _direction _direction_2 0.0001))))

(fn SetCurrentasPrevious
  (Variables|Default|SetOldParameters (CallFunction|GetCurrentParameters)))

(fn ToggleVisibility
  (bind _output_get (Variables|Default|SetVisible (not (Variables|Default|GetVisible))))
  (Rendering|SetActorHiddenInGame (not _output_get))
  (if _output_get
    (Transformation|SetActorTransform (Variables|Default|GetLast%20Visible%20Transform))
    (else
      (Variables|Default|SetLast%20Visible%20Transform (Transformation|GetActorTransform))
      (Transformation|SetActorTransform (Math|Transform|MakeTransform "0.000000,0.000000,10000.000000" "0, 0, 0" "1,1,1")))))