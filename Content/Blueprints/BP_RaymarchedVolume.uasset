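; Actor that renders a volume texture, optionally loaded from an MHD file, by raymarching with switchable lit and pure-intensity materials.
; Construction sizes the actor, bakes the transfer function curve to a texture and creates dynamic materials; BeginPlay creates raymarch resources.
; Tick propagates directional lights into a light volume, updating changed lights individually or rebuilding when over half change, the volume or clipping plane moves, or recompute is requested.
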(event EventBeginPlay
  ;[1 1 1] Creation
  (bind _outparameters (Class|RaymarchBlueprintLibrary|CreateBasicRaymarchingResources (Variables|EditorSetup|GetData%20Volume) (Variables|EditorSetup|GetALightVolume) 0 (Variables|Internal|GetTF%20Ranges) (Variables|EditorSetup|GetHalf%20Resolution%20Light%20Volume)))
  (Variables|Internal|SetRaymarch%20Resources _outparameters)
  (CallFunction|SetLitRaymarchMaterialParameters)
  (CallFunction|SetPureIntensityMaterialParameters))

(event EventTick
  (params (DeltaSeconds :type Float%20%28single-precision%29))
  (if (Variables|Internal|GetFirst%20Light%20Propagation%20Done)
    ;[0 0 0] Check if the volume was rotated or Clipping Plane moved
    (if (CallFunction|NeedsWorldUpdate)
      (Variables|Internal|SetRequestedRecompute false)
      ;[1 0.7977 0] If the volume or clipping plane moved, recalculate all lights and update clipping parameters
      (CallFunction|ResetAllLights)
      (CallFunction|SetClippingPlaneParams)
      (else
        ;[0 0 0] Count the number of lights in need of an update
        (Variables|Internal|SetUpdatedLightCount 0)
        (for _array_element (Variables|EditorSetup|GetLights%20Array)
          (if (Default|NeedsUpdate _array_element)
            (Math|Integer|IncrementInt (Variables|Internal|GetUpdatedLightCount))))
        ;[0 0 0] Check if any light wants an update
        (if (> (Variables|Internal|GetUpdatedLightCount) 0)
          ;[0 0 0] Check if more than half of lights want update
          ; If they do, do a full reset
          (if (>= (Utilities|Array|Length (Variables|EditorSetup|GetLights%20Array)) (* (Variables|Internal|GetUpdatedLightCount) 2))
            ;[1 0.7977 0] Only update lights that need it
            (for _array_element_2 (Variables|EditorSetup|GetLights%20Array)
              (bind _output_get (Variables|Internal|SetCurrentLight _array_element_2))
              (if (Default|NeedsUpdate _output_get)
                (CallFunction|UpdateLight (Variables|Internal|GetCurrentLight))))
            (else
              ;[1 0.7977 0] More than half need update -> full reset
              (CallFunction|ResetAllLights))))))
    (else
      ;[1 0.7977 0] Very first draw for each light
      (for _array_element_3 (Variables|EditorSetup|GetLights%20Array)
        (bind _lightadded (Class|RaymarchBlueprintLibrary|AddDirLighttoSingleVolume (Variables|Internal|GetRaymarch%20Resources) (Default|GetCurrent _array_element_3) true (CallFunction|GetWorldParameters)))
        ;[1 1 1] Only set the bool to true if the lights were really added (because at the very beginning, the resources for volume textures will be not usable for the first few ticks)
        (bind _output_get_2 (Variables|Internal|SetFirst%20Light%20Propagation%20Done _lightadded))
        (if _output_get_2
          (Default|SetPrevious _array_element_3 (Default|GetCurrent _array_element_3)))))))

(event Input|KeyboardEvents|R
  (params (Key :type Key%20Structure))
  ;[1 1 1] Keyboard controls
)

(event Input|KeyboardEvents|SpaceBar
  (params (Key :type Key%20Structure))
  ;[1 1 1] Keyboard controls
)

(event Input|KeyboardEvents|K
  (params (Key :type Key%20Structure))
  ;[1 1 1] Keyboard controls
)

(event Input|KeyboardEvents|H
  (params (Key :type Key%20Structure))
  ;[1 1 1] Keyboard controls
)

(event Input|KeyboardEvents|5
  (params (Key :type Key%20Structure))
  ;[1 1 1] TF Ranges Keyboard controls
)

(event Input|KeyboardEvents|6
  (params (Key :type Key%20Structure))
  ;[1 1 1] TF Ranges Keyboard controls
)

(event Input|KeyboardEvents|7
  (params (Key :type Key%20Structure))
  ;[1 1 1] TF Ranges Keyboard controls
)

(event Input|KeyboardEvents|8
  (params (Key :type Key%20Structure))
  ;[1 1 1] TF Ranges Keyboard controls
)

(event Input|KeyboardEvents|Add
  (params (Key :type Key%20Structure))
  ;[1 1 1] Keyboard controls
)

(event Input|KeyboardEvents|Subtract
  (params (Key :type Key%20Structure))
  ;[1 1 1] Keyboard controls
)

(event Input|KeyboardEvents|T
  (params (Key :type Key%20Structure))
  ;[1 1 1] Keyboard controls
)

(event Input|KeyboardEvents|U
  (params (Key :type Key%20Structure))
  ;[1 1 1] Keyboard controls
)

(event Input|KeyboardEvents|J
  (params (Key :type Key%20Structure))
  ;[1 1 1] Keyboard controls
)

(fn ConstructionScript
  (bind _intensityraymarchmaterialbase (Variables|Materials|GetIntensityRaymarchMaterialBase))
  (bind _litraymarchmaterialbase (Variables|Materials|GetLitRaymarchMaterialBase))
  (bind _mhd_file_name (Variables|EditorSetup|GetMHD%20File%20Name))
  (Utilities|FlowControl|Sequence
    (:then_0
      ;[1 1 1] Load MHD File if supplied
      (if (>= (Utilities|String|Len _mhd_file_name) 1)
        (bind _worlddimensions (Class|RaymarchBlueprintLibrary|LoadMhdIntoVolumeTextureAsset _mhd_file_name (Variables|EditorSetup|GetData%20Volume) true))
        (Variables|EditorSetup|SetVolume%20Size%20MM _worlddimensions)))
    (:then_1
      ;[1 1 1] Set size, create transfer function texture
      (CallFunction|SetSizewithArrows (* (Variables|EditorSetup|GetVolume%20Size%20MM) (Variables|EditorSetup|GetVolume%20Scale)))
      (Variables|Internal|SetTF%20Ranges (Utilities|Struct|MakeTransferFunctionRangeParameters (Variables|EditorSetup|TransferFunction|GetIntensity%20Range) (Variables|EditorSetup|TransferFunction|GetIntensity%20Cutoff) "TF_Clear" "TF_Clear"))
      (Class|RaymarchBlueprintLibrary|ColorCurvetoTexture (Variables|EditorSetup|TransferFunction|GetTF%20Curve) (Variables|EditorSetup|TransferFunction|GetTF%20Texture))
      (Variables|EditorSetup|SetVolume%20Dimensions (Class|RaymarchBlueprintLibrary|GetVolumeTextureDimensions (Variables|EditorSetup|GetData%20Volume))))
    (:then_2
      ;[1 1 1] Create dynamic material instances, set their parameters
      (bind _returnvalue (Rendering|Material|CreateDynamicMaterialInstance _intensityraymarchmaterialbase (Utilities|String|StringToName (Utilities|String|Append (Utilities|GetObjectName _intensityraymarchmaterialbase) "_Dynamic")) :!class /Script/Engine.KismetMaterialLibrary))
      (Variables|Materials|SetIntensityRaymarchMaterialDynamic _returnvalue)
      (bind _returnvalue_2 (Rendering|Material|CreateDynamicMaterialInstance (Variables|Debug|GetStaticMeshComponent) 0 _litraymarchmaterialbase (Utilities|String|StringToName (Utilities|String|Append (Utilities|GetObjectName _litraymarchmaterialbase) "_Dynamic")) :!class /Script/Engine.PrimitiveComponent))
      (Variables|Materials|SetLitRaymarchMaterialDynamic _returnvalue_2)
      (CallFunction|SetLitRaymarchMaterialParameters)
      (CallFunction|SetPureIntensityMaterialParameters))
    (:then_3
      ;[1 1 1] Set Visibility of coordinate system
      (Rendering|SetVisibility (Variables|Components|GetCoordinateSystem) (Variables|EditorSetup|GetShow%20Axis%20Arrows) true))))

(fn SetLitRaymarchMaterialParameters
  (bind _returnvalue (Math|Vector|MakeVector 1.0 1.0 1.0))
  (bind _tf_ranges (Variables|Internal|GetTF%20Ranges))
  (bind _litraymarchmaterialdynamic (Variables|Materials|GetLitRaymarchMaterialDynamic))
  (bind _data_volume (Variables|EditorSetup|GetData%20Volume))
  (bind _intensitydomain (Utilities|Struct|BreakTransferFunctionRangeParameters _tf_ranges))
  (bind _dimensions (Class|RaymarchBlueprintLibrary|GetVolumeTextureDimensions _data_volume))
  (bind _returnvalue_2 (Math|Conversions|ToVector(Float) _dimensions))
  (bind (_x _y) (Math|Vector2D|BreakVector2D _intensitydomain))
  (bind _returnvalue_3 (/ _returnvalue _returnvalue_2))
  (bind _returnvalue_4 (Math|Conversions|ToLinearColor(Vector) _returnvalue_3))
  (Utilities|FlowControl|Sequence
    (:then_0
      (Rendering|Material|SetTextureParameterValue _litraymarchmaterialdynamic "Volume" (Variables|EditorSetup|GetData%20Volume)))
    (:then_1
      (Rendering|Material|SetTextureParameterValue _litraymarchmaterialdynamic "ALightVolume" (Variables|EditorSetup|GetALightVolume)))
    (:then_2
      (Rendering|Material|SetTextureParameterValue _litraymarchmaterialdynamic "TF" (Variables|EditorSetup|TransferFunction|GetTF%20Texture)))
    (:then_3
      (Rendering|Material|SetVectorParameterValue _litraymarchmaterialdynamic "TFIntensityDomain" (Math|Conversions|ToLinearColor(Vector) (Math|Vector|MakeVector _x _y 0.0)) :!class /Script/Engine.MaterialInstanceDynamic))
    (:then_4
      (Rendering|Material|SetScalarParameterValue _litraymarchmaterialdynamic "Plane Alignment" (Variables|RaymarcherTweaking|GetPlaneAlignment) :!class /Script/Engine.MaterialInstanceDynamic))
    (:then_5
      (Rendering|Material|SetVectorParameterValue _litraymarchmaterialdynamic "VoxelSizeTex" _returnvalue_4 :!class /Script/Engine.MaterialInstanceDynamic))
    (:then_6
      (Rendering|Material|SetScalarParameterValue _litraymarchmaterialdynamic "SamplingStepSize" (/ (Class|KismetMathLibrary|LinearColorGetMin _returnvalue_4) (Variables|RaymarcherTweaking|GetVolumeSamplingRate)) :!class /Script/Engine.MaterialInstanceDynamic))))

(fn UpdateLight
  (params (Light :type BP%20Raymarching%20Light%20Object%20Reference%20%28by%20ref%29))
  (bind _output_get (Variables|Internal|SetCurrentLight Light))
  (bind _locallightdir (Class|RaymarchBlueprintLibrary|ChangeDirLightinSingleVolume (Variables|Internal|GetRaymarch%20Resources) (Default|GetPrevious _output_get) (Default|GetCurrent _output_get) (CallFunction|GetWorldParameters)))
  (Default|SetCurrentasPrevious (Variables|Internal|GetCurrentLight))
  (CallFunction|SetArrowLocalLight _locallightdir))

(fn GetClippingParameters
  (bind _clipping_plane (Variables|EditorSetup|GetClipping%20Plane))
  (Utilities|IsValid _clipping_plane
    (:Is%20Valid
      (return (Default|GetCurrentParameters _clipping_plane)))
    (:Is%20Not%20Valid
      (return (Utilities|Struct|MakeClippingPlaneParameters "0.000000, 0,10000.000000" "0, 0,-1.000000")))))

(fn SetPureIntensityMaterialParameters
  (bind _returnvalue (Math|Vector|MakeVector 1.0 1.0 1.0))
  (bind _intensityraymarchmaterialdynamic (Variables|Materials|GetIntensityRaymarchMaterialDynamic))
  (bind _data_volume (Variables|EditorSetup|GetData%20Volume))
  (bind _dimensions (Class|RaymarchBlueprintLibrary|GetVolumeTextureDimensions _data_volume))
  (bind _returnvalue_2 (Math|Conversions|ToVector(Float) _dimensions))
  (bind _returnvalue_3 (/ _returnvalue _returnvalue_2))
  (bind _returnvalue_4 (Math|Conversions|ToLinearColor(Vector) _returnvalue_3))
  (Utilities|FlowControl|Sequence
    (:then_0
      (Rendering|Material|SetTextureParameterValue _intensityraymarchmaterialdynamic "Volume" (Variables|EditorSetup|GetData%20Volume)))
    (:then_1
      (Rendering|Material|SetScalarParameterValue _intensityraymarchmaterialdynamic "SamplingStepSize" (/ (Class|KismetMathLibrary|LinearColorGetMin _returnvalue_4) (Variables|RaymarcherTweaking|GetVolumeSamplingRate)) :!class /Script/Engine.MaterialInstanceDynamic))
    (:then_2
      (Rendering|Material|SetVectorParameterValue _intensityraymarchmaterialdynamic "VoxelSizeTex" _returnvalue_4 :!class /Script/Engine.MaterialInstanceDynamic))))

(fn GetClippingParametersLocal
  (bind _clippingparameters (CallFunction|GetClippingParameters))
  (bind _returnvalue (Transformation|GetActorScale3D))
  (bind _returnvalue_2 (Transformation|GetActorTransform))
  (bind (_center _direction) (Utilities|Struct|BreakClippingPlaneParameters _clippingparameters))
  (bind _returnvalue_3 (Math|Transform|InverseTransformLocation _returnvalue_2 _center))
  (bind _returnvalue_4 (Math|Transform|InverseTransformDirection _returnvalue_2 _direction))
  (bind _returnvalue_5 (+ _returnvalue_3 0.5))
  (bind _returnvalue_6 (* _returnvalue_4 _returnvalue))
  (bind _returnvalue_7 (Math|Vector|Normalize _returnvalue_6))
  (bind (_x _y _z) (Math|Vector|BreakVector _returnvalue_7))
  (return _returnvalue_5 _returnvalue_7 (Utilities|Struct|MakeLinearColor _x _y _z (Math|Vector|DotProduct _returnvalue_5 _returnvalue_7))))

(fn SetSizewithArrows
  (params (NewSize :type Vector))
  (bind _staticmeshcomponent (Variables|Debug|GetStaticMeshComponent))
  (bind _returnvalue (Transformation|GetWorldScale _staticmeshcomponent))
  (bind (_x _y _z) (Math|Vector|BreakVector _returnvalue))
  (bind _returnvalue_2 (Math|Float|Sqrt _x))
  (bind _returnvalue_3 (Math|Float|Sqrt _z))
  (bind _returnvalue_4 (Math|Float|Sqrt _y))
  (bind _returnvalue_5 (+ _returnvalue_4 _returnvalue_3))
  (bind _returnvalue_6 (+ _returnvalue_2 _returnvalue_5))
  (bind _returnvalue_7 (/ _returnvalue_6 0.5))
  (Transformation|SetActorRelativeScale3D NewSize)
  (Transformation|SetRelativeScale3D (Variables|Components|GetArrowX) (Math|Vector|MakeVector _x _returnvalue_7 _returnvalue_7))
  (Transformation|SetRelativeScale3D (Variables|Components|GetArrowY) (Math|Vector|MakeVector _y _returnvalue_7 _returnvalue_7))
  (Transformation|SetRelativeScale3D (Variables|Components|GetArrowZ) (Math|Vector|MakeVector _z _returnvalue_7 _returnvalue_7)))

(fn SetArrowLocalLight
  (params (Direction :type Vector))
  (Transformation|SetRelativeRotation (Variables|Components|GetArrowLocalLight) (Math|Conversions|RotationFromXVector Direction) false false))

(fn GetWorldParameters
  (return (Utilities|Struct|MakeRaymarchWorldParameters (Transformation|GetActorTransform) (CallFunction|GetClippingParameters))))

(fn NeedsWorldUpdate
  (bind _worldparams (CallFunction|GetWorldParameters))
  (bind _oldworldparameters (Variables|Internal|GetOldWorldParameters))
  (bind (_volumetransform _clippingplaneparameters) (Utilities|Struct|BreakRaymarchWorldParameters _oldworldparameters))
  (bind (_volumetransform_2 _clippingplaneparameters_2) (Utilities|Struct|BreakRaymarchWorldParameters _worldparams))
  (bind (_center _direction) (Utilities|Struct|BreakClippingPlaneParameters _clippingplaneparameters_2))
  (bind (_center_2 _direction_2) (Utilities|Struct|BreakClippingPlaneParameters _clippingplaneparameters))
  (return (Math|Boolean|ORBoolean (not (Class|KismetMathLibrary|NearlyEqualTransformTransform _volumetransform_2 _volumetransform 0.01 0.01 0.01)) (Math|Vector|NotEqual(Vector) _center _center_2 0.01) (Math|Vector|NotEqual(Vector) _direction _direction_2 0.01) (Variables|Internal|GetRequestedRecompute))))

(fn ResetAllLights
  ;[1 0.7977 0] Reset all light volumes to zero and add all lights with new rotation
  (Variables|Internal|SetOldWorldParameters (CallFunction|GetWorldParameters))
  (Class|RaymarchBlueprintLibrary|ClearResourceLightVolumes (Variables|Internal|GetRaymarch%20Resources) 0.0)
  (for _array_element (Variables|EditorSetup|GetLights%20Array)
    (bind _locallightdir (Class|RaymarchBlueprintLibrary|AddDirLighttoSingleVolume (Variables|Internal|GetRaymarch%20Resources) (Default|GetCurrent _array_element) true (CallFunction|GetWorldParameters)))
    (Default|SetCurrentasPrevious _array_element)
    (CallFunction|SetArrowLocalLight _locallightdir)))

(fn SetClippingPlaneParams
  (bind (_centerlocal _directionlocal _hnf) (CallFunction|GetClippingParametersLocal))
  (bind _litraymarchmaterialdynamic (Variables|Materials|GetLitRaymarchMaterialDynamic))
  (bind _intensityraymarchmaterialdynamic (Variables|Materials|GetIntensityRaymarchMaterialDynamic))
  (bind _returnvalue (Math|Conversions|ToLinearColor(Vector) _directionlocal))
  (bind _returnvalue_2 (Math|Conversions|ToLinearColor(Vector) _centerlocal))
  ;[1 1 1] Set Shader parameters relating to clipping plane
  (Rendering|Material|SetVectorParameterValue _litraymarchmaterialdynamic "ClippingCenter" _returnvalue_2 :!class /Script/Engine.MaterialInstanceDynamic)
  (Rendering|Material|SetVectorParameterValue _litraymarchmaterialdynamic "ClippingDirection" _returnvalue :!class /Script/Engine.MaterialInstanceDynamic)
  (Rendering|Material|SetVectorParameterValue _litraymarchmaterialdynamic "ClippingPlane" _hnf :!class /Script/Engine.MaterialInstanceDynamic)
  (Rendering|Material|SetVectorParameterValue _intensityraymarchmaterialdynamic "ClippingCenter" _returnvalue_2 :!class /Script/Engine.MaterialInstanceDynamic)
  (Rendering|Material|SetVectorParameterValue _intensityraymarchmaterialdynamic "ClippingDirection" _returnvalue :!class /Script/Engine.MaterialInstanceDynamic)
  (Rendering|Material|SetVectorParameterValue _intensityraymarchmaterialdynamic "ClippingPlane" _hnf :!class /Script/Engine.MaterialInstanceDynamic))

(fn NeedsWorldUpdateNew
  (for _array_element (Variables|EditorSetup|GetLights%20Array)
    (if (Default|NeedsUpdate _array_element)
      (return true)))
  (if (Default|NeedsUpdate (Variables|EditorSetup|GetClipping%20Plane))
    (return true)
    (else
      (return false))))

(fn ChangeTFParameters
  (params (NewRanges :type Transfer%20Function%20Range%20Parameters%20Structure))
  (Variables|Internal|SetTF%20Ranges NewRanges)
  (bind _outresources (Class|RaymarchBlueprintLibrary|ChangeTFinResources (Variables|Internal|GetRaymarch%20Resources) (Variables|EditorSetup|TransferFunction|GetTF%20Texture) (Variables|Internal|GetTF%20Ranges)))
  (Variables|Internal|SetRaymarch%20Resources _outresources)
  (Rendering|Material|SetVectorParameterValue (Variables|Materials|GetLitRaymarchMaterialDynamic) "TFIntensityDomain" (Math|Conversions|ToLinearColor(Vector) (Math|Vector|MakeVector (.X (Math|Vector2D|BreakVector2D (.IntensityDomain (Utilities|Struct|BreakTransferFunctionRangeParameters (Variables|Internal|GetTF%20Ranges))))) (.Y (Math|Vector2D|BreakVector2D (.IntensityDomain (Utilities|Struct|BreakTransferFunctionRangeParameters (Variables|Internal|GetTF%20Ranges))))) 0.0)) :!class /Script/Engine.MaterialInstanceDynamic)
  (Variables|Internal|SetRequestedRecompute true))

(fn SwitchRenderer
  (bind _output_get (Variables|Materials|SetLit%20Raymarching (not (Variables|Materials|GetLit%20Raymarching))))
  (if _output_get
    (Rendering|Material|SetMaterial (Variables|Debug|GetStaticMeshComponent) 0 (Variables|Materials|GetLitRaymarchMaterialDynamic))
    (else
      (Rendering|Material|SetMaterial (Variables|Debug|GetStaticMeshComponent) 0 (Variables|Materials|GetIntensityRaymarchMaterialDynamic)))))

(fn UpdateVolume
  (params (New%20Volume :type Volume%20Texture%20Object%20Reference) (New%20Size :type Vector) (New%20Rel.%20Center%20Position :type Vector) (New%20Rel.%20Rotation :type Rotator))
  (bind _dimensions (Class|RaymarchBlueprintLibrary|GetVolumeTextureDimensions New%20Volume))
  (bind _volume_scale (Variables|EditorSetup|GetVolume%20Scale))
  (bind _returnvalue (* New%20Size _volume_scale))
  (Utilities|FlowControl|Sequence
    (:then_0
      (Variables|EditorSetup|SetData%20Volume New%20Volume)
      (if (Math|Vector|NotEqual(Vector) (Math|Conversions|ToVector(Float) (Variables|EditorSetup|GetVolume%20Dimensions)) (Math|Conversions|ToVector(Float) _dimensions) 0.0001)
        (Variables|EditorSetup|SetVolume%20Dimensions _dimensions)))
    (:then_1
      (bind _outparameters (Class|RaymarchBlueprintLibrary|CreateBasicRaymarchingResources (Variables|EditorSetup|GetData%20Volume) (Variables|EditorSetup|GetALightVolume) (Variables|EditorSetup|TransferFunction|GetTF%20Texture) (Variables|Internal|GetTF%20Ranges) (Variables|EditorSetup|GetHalf%20Resolution%20Light%20Volume)))
      (Variables|Internal|SetRaymarch%20Resources _outparameters)
      (Variables|Internal|SetRequestedRecompute true)
      (CallFunction|SetLitRaymarchMaterialParameters)
      (CallFunction|SetPureIntensityMaterialParameters))
    (:then_2
      (CallFunction|SetSizewithArrows _returnvalue)
      (Transformation|SetActorRelativeTransform (Math|Transform|MakeTransform New%20Rel.%20Center%20Position New%20Rel.%20Rotation _returnvalue) false true))))

(fn SetTFRange
  (params (Range :type Vector%202D%20Structure :default "(X=0.000000,Y=1.000000)"))
  (bind _tf_ranges (Variables|Internal|GetTF%20Ranges))
  (CallFunction|ChangeTFParameters (Utilities|Struct|MakeTransferFunctionRangeParameters Range Range (.lowcutmode _tf_ranges) (.highcutmode _tf_ranges))))

(fn GetTFRange
  (return (.intensitydomain (Variables|Internal|GetTF%20Ranges))))