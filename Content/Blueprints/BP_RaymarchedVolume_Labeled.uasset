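; Raymarched volume actor that adds a paintable label volume on top of its parent's data volume rendering.
; It sizes the label texture to the data volume at BeginPlay and re-initializes it when UpdateVolume receives different dimensions.
; Parent overrides feed the label texture into the lit and intensity raymarch materials.
; Functions paint labeled spheres in world or local space, clear the labels, and toggle their display in both materials.
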(event EventBeginPlay
  (Development|PrintString (Utilities|String|ToString(Integer) (Class|RaymarchBlueprintLibrary|GetVolumeTextureDimensions (Variables|Default|GetData%20Volume))) true true "(R=1.000000,G=0.137129,B=0.047459,A=1.000000)" 2e+01)
  ;[1 1 1] Create labeling volume and then call parent's beginplay
  ; (That one calls setting all params to materials)
  (Class|LabelVolumeLibrary|InitLabelingVolume (Variables|EditorSetup|Labeling|GetLabel%20Volume) (Class|RaymarchBlueprintLibrary|GetVolumeTextureDimensions (Variables|Default|GetData%20Volume)))
  (|CallParentFunction)
  (Rendering|Material|SetTextureParameterValue (Variables|Default|GetLitRaymarchMaterialDynamic) "LabelVolume" (Variables|EditorSetup|Labeling|GetLabel%20Volume)))

(event Collision|EventActorBeginOverlap
  (params (OtherActor :type Actor%20Object%20Reference)))

(event EventTick
  (params (DeltaSeconds :type Float%20%28single-precision%29))
  (|CallParentFunction DeltaSeconds) ; This node is disabled and will not be called.\nDrag off pins to build functionality.
)

(event EventSetPureIntensityMaterialParameters
  (bind _litraymarchmaterialdynamic (Variables|Default|GetLitRaymarchMaterialDynamic))
  (|CallParentFunction)
  (Rendering|Material|SetTextureParameterValue _litraymarchmaterialdynamic "LabelVolume" (Variables|EditorSetup|Labeling|GetLabel%20Volume))
  (Rendering|Material|SetScalarParameterValue _litraymarchmaterialdynamic "LabelVolumeEnabled" 1.0 :!class /Script/Engine.MaterialInstanceDynamic))

(event EventSetLitRaymarchMaterialParameters
  (bind _intensityraymarchmaterialdynamic (Variables|Default|GetIntensityRaymarchMaterialDynamic))
  (|CallParentFunction)
  (Rendering|Material|SetTextureParameterValue _intensityraymarchmaterialdynamic "LabelVolume" (Variables|EditorSetup|Labeling|GetLabel%20Volume))
  (Rendering|Material|SetScalarParameterValue _intensityraymarchmaterialdynamic "LabelVolumeEnabled" 1.0 :!class /Script/Engine.MaterialInstanceDynamic))

(event EventUpdateVolume
  (params (New%20Volume :type Volume%20Texture%20Object%20Reference) (New%20Size :type Vector :default "0, 0, 0") (New%20Rel.%20Center%20Position :type Vector :default "0, 0, 0") (New%20Rel.%20Rotation :type Rotator :default "0, 0, 0"))
  (bind _dimensions (Class|RaymarchBlueprintLibrary|GetVolumeTextureDimensions New%20Volume))
  (if (Math|Vector|NotEqual(Vector) (Math|Conversions|ToVector(Float) (Variables|Default|GetVolume%20Dimensions)) (Math|Conversions|ToVector(Float) _dimensions) 0.0001)
    (Class|LabelVolumeLibrary|InitLabelingVolume (Variables|EditorSetup|Labeling|GetLabel%20Volume) _dimensions))
  (|CallParentFunction New%20Volume New%20Size New%20Rel.%20Center%20Position New%20Rel.%20Rotation))

(fn ConstructionScript
  (|CallParentFunction)
  (Rendering|Material|SetTextureParameterValue (Variables|Default|GetLitRaymarchMaterialDynamic) "Volume" (Variables|Default|GetData%20Volume))
  (Rendering|Material|SetTextureParameterValue (Variables|Default|GetLitRaymarchMaterialDynamic) "LabelVolume" (Variables|EditorSetup|Labeling|GetLabel%20Volume)))

(fn ToggleLabelVolume
  (bind _output_get (Variables|Labeling|SetLabel%20Volume%20Enabled (not (Variables|Labeling|GetLabel%20Volume%20Enabled))))
  (Rendering|Material|SetScalarParameterValue (Variables|Default|GetLitRaymarchMaterialDynamic) "LabelVolumeEnabled" (Math|Conversions|ToFloat(Boolean) _output_get) :!class /Script/Engine.MaterialInstanceDynamic)
  (Rendering|Material|SetScalarParameterValue (Variables|Default|GetIntensityRaymarchMaterialDynamic) "LabelVolumeEnabled" (Math|Conversions|ToFloat(Boolean) _output_get) :!class /Script/Engine.MaterialInstanceDynamic))

(fn LabelSphereWorld
  (params (World%20Position :type Vector) (Sphere%20World%20Radius :type Float%20%28single-precision%29) (Label :type FSurgeryLabel%20Enum :default "SL_Clear"))
  (Class|LabelVolumeLibrary|LabelSphereinVolumeWorld (Variables|EditorSetup|Labeling|GetLabel%20Volume) World%20Position Sphere%20World%20Radius (CallFunction|GetWorldParameters) Label))

(fn ClearLabelVolume
  (Class|RaymarchBlueprintLibrary|ClearVolumeTexture (Variables|EditorSetup|Labeling|GetLabel%20Volume) 0.0))

(fn LabelSphereLocal
  (params (Local%20Center :type Vector) (Local%20Radius :type Float%20%28single-precision%29) (Label :type FSurgeryLabel%20Enum :default "SL_Clear"))
  (Class|LabelVolumeLibrary|LabelSphereinVolumeLocal (Variables|EditorSetup|Labeling|GetLabel%20Volume) Local%20Center Local%20Radius Label))